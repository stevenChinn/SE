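; Pearl is a pet character Blueprint that follows the player around the level.
; Looping timers measure player distance, issue AI move orders when not close, and teleport Pearl to a random navigable point near the player when too far away.
; A sphere overlap with the player plays or reverses a timeline that ramps Pearl's walk speed.
; The bite attack is work in progress, playing an animation and printing a debug message.
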(event `self.Sphere.OnComponentBeginOverlap`
  (params (OverlappedComponent :type "PrimitiveComponent Object Reference") (OtherActor :type "Actor Object Reference") (OtherComp :type "PrimitiveComponent Object Reference") (OtherBodyIndex :type Integer) (bFromSweep :type Boolean) (SweepResult :type "HitResult Structure (by ref)"))
  (cast `/Game/Blueprints/ThirdPersonBP/Blueprints/ThirdPersonCharacter` OtherActor)
  (bind (_direction _speed_slide) (`Timeline|Speed Ramp` :!via `PlayFromStart` :!label _label)
    (:`Update`
      (set `CharacterMovementComponent.MaxWalkSpeed` _speed_slide (`self.CharacterMovement`)))))

(event `self.Sphere.OnComponentEndOverlap`
  (params (OverlappedComponent :type "PrimitiveComponent Object Reference") (OtherActor :type "Actor Object Reference") (OtherComp :type "PrimitiveComponent Object Reference") (OtherBodyIndex :type Integer))
  (cast `/Game/Blueprints/ThirdPersonBP/Blueprints/ThirdPersonCharacter` OtherActor)
  (goto _label :!via `ReverseFromEnd`))

(event `self.ReceiveBeginPlay`
  (`parent.ReceiveBeginPlay`)
  (bind _asthird_person_character (cast `/Game/Blueprints/ThirdPersonBP/Blueprints/ThirdPersonCharacter` (`GameplayStatics.GetPlayerCharacter` 0)))
  (set `self.PlayerReference` _asthird_person_character)
  (`KismetSystemLibrary.K2_SetTimerDelegate` (delegate `DistanceToPlayer`) 0.33 true)
  (`KismetSystemLibrary.K2_SetTimerDelegate` (delegate `MovePearlToPlayer`) 1.0 true)
  (`KismetSystemLibrary.K2_SetTimerDelegate` (delegate `PearlStuck?`) 10.0 true))

(event `DistanceToPlayer`
  (set `self.DistancePearlToPlayer` (`self.GetDistanceTo` (`self.PlayerReference`))))

(event `MovePearlToPlayer`
  (bind _playerreference (`self.PlayerReference`))
  (if (not (<= (`self.DistancePearlToPlayer`) 100.0))
    (`|AIMoveTo` self (`self.K2_GetActorLocation` _playerreference) _playerreference 20.0)))

(event `PearlStuck?`
  (if (>= (`self.DistancePearlToPlayer`) 3500.0)
    (`SceneComponent.K2_SetWorldLocation` (`self.CapsuleComponent`) (`NavigationSystemV1.K2_GetRandomLocationInNavigableRadius` (`self.K2_GetActorLocation` (`self.PlayerReference`)) 1000.0 null null) false false)))

(event `self.ReceiveAnyDamage`
  (params (Damage :type "Float (single-precision)") (DamageType :type "DamageType Object Reference") (InstigatedBy :type "Controller Object Reference") (DamageCauser :type "Actor Object Reference")))

(fn `AttackTarget`
  ;[1 1 1] Pearl attack functionality - WIP
  (if true
    (`SkeletalMeshComponent.PlayAnimation` (`self.Mesh`) null false)
    (`KismetSystemLibrary.PrintString` "Pearl: Bite")))

(fn `MoveToTarget`
  (`self.MoveToTarget`)
  (`self.AttackTarget`))

(fn `UserConstructionScript`
  (`parent.UserConstructionScript`))