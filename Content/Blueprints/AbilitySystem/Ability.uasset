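; Ability actor, apparently a base with an empty ActivateEffect hook, that runs the casting flow for an ability in the player's action bar system.
; On BeginPlay it snaps to the caster's hand socket and, for timed abilities, shows a cast bar, flags the player as casting and binds to its success event.
; Instant abilities call CastAbility directly, which prints the name, clears the flag and detaches the actor.
; InterruptCast destroys it.
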(event `self.ReceiveBeginPlay`
  (`self.K2_AttachToComponent` (`Character.Mesh` (`self.Caster`)) "hand_rSocket" "SnapToTarget" "SnapToTarget" "SnapToTarget")
  (bind _asthird_person_character (cast `/Game/Blueprints/ThirdPersonBP/Blueprints/ThirdPersonCharacter` (`GameplayStatics.GetPlayerCharacter` 0)))
  (set `self.PlayerRef` _asthird_person_character)
  (bind _asthird_person_character_2 (cast `/Game/Blueprints/ThirdPersonBP/Blueprints/ThirdPersonCharacter` (`GameplayStatics.GetPlayerCharacter` 0)))
  (set `self.Action Bar UI Ref` (`/Game/Blueprints/ThirdPersonBP/Blueprints/ThirdPersonCharacter.UI_Ref` _asthird_person_character_2))
  (`self.Begin Casting`))

(fn `ActivateEffect`)

(fn `Begin Casting`
  (bind (_abilitydetails_name _abilitydetails_description _abilitydetails_thumbnail _abilitydetails_cost _abilitydetails_cooldown _abilitydetails_casttime) (break `/Game/Blueprints/AbilitySystem/AbilityDetailsStructure` (`self.AbilityDetails`)))
  (if (> _abilitydetails_casttime 0.0)
    (bind _castbar (`/Game/Blueprints/UI/UI_Player/Player_UI.DisplayCastBar` (`self.Action Bar UI Ref`) self))
    (if (`Widget.IsVisible` _castbar)
      (bind _asthird_person_character (cast `/Game/Blueprints/ThirdPersonBP/Blueprints/ThirdPersonCharacter` (`GameplayStatics.GetPlayerCharacter` 0)))
      (set `/Game/Blueprints/ThirdPersonBP/Blueprints/ThirdPersonCharacter.IsCasting` true _asthird_person_character)
      (add `/Game/Blueprints/UI/UI_Player/CastBar_UI.CastSuccessful` _castbar (`|CreateDelegate` :!event `CastAbility`)))
    (else
      (`self.CastAbility`))))

(fn `CastAbility`
  (`KismetSystemLibrary.PrintString` (`KismetTextLibrary.Conv_TextToString` (`.Name_2_742AFD324C7840476E2CCBA9FDB6D855` (break `/Game/Blueprints/AbilitySystem/AbilityDetailsStructure` (`self.AbilityDetails`)))))
  (bind _asthird_person_character (cast `/Game/Blueprints/ThirdPersonBP/Blueprints/ThirdPersonCharacter` (`GameplayStatics.GetPlayerCharacter` 0)))
  (set `/Game/Blueprints/ThirdPersonBP/Blueprints/ThirdPersonCharacter.IsCasting` false _asthird_person_character)
  (`self.K2_DetachFromActor` "KeepWorld" "KeepWorld" "KeepWorld"))

(fn `InterruptCast`
  (`self.K2_DestroyActor`)
  (`KismetSystemLibrary.PrintString` "Cast Interrupted"))

(fn `UserConstructionScript`)