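; Base buff ability actor that runs for a set duration, with empty TickBuff and ClearBuff hooks.
; On cast it destroys itself if another actor of its class is attached to the caster, sets its lifespan from the ability duration, registers with the action bar buff UI and starts a looping tick timer.
; BeginPlay plays an AoE montage on the player mesh, and EndPlay broadcasts the buff's removal.
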(event `self.CastAbility`
  (bind (_abilitydetails_name _abilitydetails_description _abilitydetails_thumbnail _abilitydetails_cost _abilitydetails_cooldown _abilitydetails_casttime _abilitydetails_duration) (break `/Game/Blueprints/AbilitySystem/AbilityDetailsStructure` (`self.AbilityDetails`)))
  (`self.ClearDuplicate`)
  (`self.SetLifeSpan` _abilitydetails_duration)
  (`self.ApplyBuff`)
  (bind _returnvalue (`KismetSystemLibrary.K2_SetTimerDelegate` (delegate `TickBuff`) (`self.TickRate`) true))
  (set `self.BuffTickTimer` _returnvalue))

(event `TickBuff`)

(event `self.ReceiveBeginPlay`
  (`parent.ReceiveBeginPlay`)
  (`|PlayMontage` (`Character.Mesh` (`self.PlayerRef`)) "/Game/SampleContent/TempSampleAnimations/Aoe_Montage.Aoe_Montage"))

(event `self.ReceiveEndPlay`
  (params (EndPlayReason :type "EEndPlayReason Enum" :default "Destroyed"))
  (`self.BuffRemoved`))

(fn `ApplyBuff`
  (`/Game/Blueprints/UI/UI_Player/BuffArray_UI.AddBuffToUI` (`/Game/Blueprints/UI/UI_Player/Player_UI.BuffArray_UI` (`self.Action Bar UI Ref`)) self))

(fn `ClearBuff`)

(fn `ClearDuplicate`
  (for _array_element (`self.GetAttachedActors` (`self.Caster`) true)
    (if (and (== (`GameplayStatics.GetObjectClass` _array_element) (`GameplayStatics.GetObjectClass` self)) (!= _array_element self))
      (`self.K2_DestroyActor`))))

(fn `UserConstructionScript`
  (`parent.UserConstructionScript`))