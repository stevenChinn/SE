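; AbilityDebuff is an ability actor for timed debuffs on the player controller's current target, apparently a base for specific debuffs.
; On BeginPlay it plays an AoE montage on the player mesh.
; CastAbility destroys itself if the target already carries the same class, sets lifespan from the ability duration, attaches to the target and refreshes the target frame.
; A looping timer calls DebuffTick, an empty hook here.
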(event `self.CastAbility`
  (`parent.CastAbility`)
  (`self.ClearDuplicates`)
  (`self.SetLifeSpan` (`.Duration_16_855CA2944845C2B4262B60BD3402204C` (break `/Game/Blueprints/AbilitySystem/AbilityDetailsStructure` (`self.AbilityDetails`))))
  (`self.ApplyDebuff`)
  (bind _returnvalue (`KismetSystemLibrary.K2_SetTimerDelegate` (delegate `DebuffTick`) (`self.TickRate`) true))
  (set `self.DebuffTickTimer` _returnvalue))

(event `DebuffTick`)

(event `self.ReceiveBeginPlay`
  (`parent.ReceiveBeginPlay`)
  (`|PlayMontage` (`Character.Mesh` (`self.PlayerRef`)) "/Game/SampleContent/TempSampleAnimations/Aoe_Montage.Aoe_Montage"))

(fn `ApplyDebuff`
  (bind _asnew_player_controller (cast `/Game/Blueprints/ThirdPersonBP/Blueprints/NewPlayerController` (`GameplayStatics.GetPlayerController` 0)))
  (`self.K2_AttachToActor` self (`/Game/Blueprints/ThirdPersonBP/Blueprints/NewPlayerController.CurrentTarget` _asnew_player_controller) "None" "SnapToTarget" "SnapToTarget" "SnapToTarget" true)
  (`/Game/Blueprints/UI/UI_Target/Targetframe.UpdateTargetUI` (`/Game/Blueprints/UI/UI_Player/Player_UI.Targetframe` (`self.Action Bar UI Ref`))))

(fn `ClearDuplicates`
  (bind _asnew_player_controller (cast `/Game/Blueprints/ThirdPersonBP/Blueprints/NewPlayerController` (`GameplayStatics.GetPlayerController` 0)))
  (for _array_element (`self.GetAttachedActors` (`/Game/Blueprints/ThirdPersonBP/Blueprints/NewPlayerController.CurrentTarget` _asnew_player_controller) true)
    (if (and (== (`GameplayStatics.GetObjectClass` _array_element) (`GameplayStatics.GetObjectClass` self)) (!= _array_element self))
      (`self.K2_DestroyActor`))))

(fn `UserConstructionScript`
  (`parent.UserConstructionScript`))