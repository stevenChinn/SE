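; Ability actor for projectile spells, extending a parent ability class with a homing launch and player cast animations.
; On BeginPlay, targeted abilities turn the player toward the current target, set a short lifespan and play the fireball montage; untargeted ones only play an AoE montage.
; Instant casts, or CastAbility for timed casts, play the montage's EndCast section, set homing on the target's capsule and immediately call ActivateEffect to start projectile movement.
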(event `self.ReceiveBeginPlay`
  (bind _playerref (`self.PlayerRef`))
  (bind (_returnvalue_roll _returnvalue_pitch) (`KismetMathLibrary.BreakRotator` (`self.K2_GetActorRotation` _playerref)))
  (bind _mesh (`Character.Mesh` (`self.PlayerRef`)))
  (bind (_returnvalue_roll_2 _returnvalue_pitch_2 _returnvalue_yaw) (`KismetMathLibrary.BreakRotator` (`KismetMathLibrary.FindLookAtRotation` (`self.K2_GetActorLocation` (`self.PlayerRef`)) (`self.K2_GetActorLocation` (`/Game/Blueprints/ThirdPersonBP/Blueprints/NewPlayerController.CurrentTarget` (`self.PlayerControllerRef`))))))
  (`parent.ReceiveBeginPlay`)
  (bind _asnew_player_controller (cast `/Game/Blueprints/ThirdPersonBP/Blueprints/NewPlayerController` (`GameplayStatics.GetPlayerController` 0)))
  (set `self.PlayerControllerRef` _asnew_player_controller)
  (if (`.RequiresTarget_40_E1ADF81B40C1BEB31FEE0192F24D50CA` (break `/Game/Blueprints/AbilitySystem/AbilityDetailsStructure` (`self.AbilityDetails`)))
    (`self.K2_SetActorRotation` _playerref (`KismetMathLibrary.MakeRotator` _returnvalue_roll _returnvalue_pitch _returnvalue_yaw) false)
    (`self.SetLifeSpan` 5.0)
    (if (> (`.CastTime_14_2ADBB90C48484617A0599C829A877BBB` (break `/Game/Blueprints/AbilitySystem/AbilityDetailsStructure` (`self.AbilityDetails`))) 0.0)
      (`|PlayMontage` _mesh "/Game/SampleContent/TempSampleAnimations/Fireball_Montage.Fireball_Montage"
        (:`then`
          (set `ProjectileMovementComponent.HomingTargetComponent` (`Character.CapsuleComponent` (`self.ProjectilesTarget`)) (`self.ProjectileMovement`))))
      (else
        (`|PlayMontage` _mesh "/Game/SampleContent/TempSampleAnimations/Fireball_Montage.Fireball_Montage" 1.5 0.0 "EndCast" :!label _label
          (:`then`
            (bind _projectilestarget (`self.ProjectilesTarget`)
              (:`then`
                (set `ProjectileMovementComponent.HomingTargetComponent` (`Character.CapsuleComponent` _projectilestarget) (`self.ProjectileMovement`)))
              (:`else`
                _))
            (`self.ActivateEffect`)))))
    (else
      (`|PlayMontage` _mesh "/Game/SampleContent/TempSampleAnimations/Aoe_Montage.Aoe_Montage" 1.5))))

(event `self.CastAbility`
  (`parent.CastAbility`)
  (goto _label))

(event `self.ActivateEffect`
  (`parent.ActivateEffect`)
  (`ActorComponent.Activate` (`self.ProjectileMovement`) false))

(fn `UserConstructionScript`
  (`parent.UserConstructionScript`))