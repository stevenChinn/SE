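; Traffic car that drives along the Route_4 spline and acts as a hazard to the player.
; On BeginPlay it finds the route actor, then a timeline scaled by TimeToComplete moves it by spline distance, using world location but local rotation.
; Tick spins four wheel components at RotateSpeed, independent of the timeline.
; Overlapping the Kill component calls UpdateHealth on the player's ThirdPersonCharacter with a fixed amount.
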(event `self.ReceiveTick`
  (params (DeltaSeconds :type "Float (single-precision)"))
  (`|ExecutionSequence`
    (:`then_0`
      (`SceneComponent.K2_AddRelativeRotation` (`|MakeArray` (`self.Tire_Centered_Wheel_C2`) (`self.Tire_Centered_Wheel_C3`) :!type "SceneComponent Object Reference") (`KismetMathLibrary.MakeRotator` (`self.RotateSpeed`)) true false))
    (:`then_1`
      (`SceneComponent.K2_AddRelativeRotation` (`|MakeArray` (`self.Tire_Centered_Wheel_C`) (`self.Tire_Centered_Wheel_C1`) :!type "SceneComponent Object Reference") (`KismetMathLibrary.MakeRotator` (`self.RotateSpeed-`)) true false))))

(event `self.ReceiveBeginPlay`
  (`|ExecutionSequence`
    (:`then_0`
      (bind _returnvalue (`GameplayStatics.GetActorOfClass` "/Game/Blueprints/Traffic/Route_4.Route_4_C"))
      (set `self.Spline REF` _returnvalue)
      (`self.Move Object`))))

(event `Move Object`
  (bind _spline (`/Game/Blueprints/Traffic/Route_4.Spline` (`self.Spline REF`)))
  (`TimelineComponent.SetPlayRate` (`self.Move Object T`) (/ 1.0 (`self.TimeToComplete`)))
  (bind (_direction _move_track) (`Timeline|Move Object T`)
    (:`Update`
      (bind _returnvalue (`KismetMathLibrary.Lerp` 0.0 (`SplineComponent.GetSplineLength` (`/Game/Blueprints/Traffic/Route_4.Spline` (`self.Spline REF`))) _move_track))
      (`self.K2_SetActorTransform` (`KismetMathLibrary.MakeTransform` (`SplineComponent.GetLocationAtDistanceAlongSpline` _spline _returnvalue "World") (`SplineComponent.GetRotationAtDistanceAlongSpline` _spline _returnvalue "Local"))))))

(event `self.Kill.OnComponentBeginOverlap`
  (params (OverlappedComponent :type "PrimitiveComponent Object Reference") (OtherActor :type "Actor Object Reference") (OtherComp :type "PrimitiveComponent Object Reference") (OtherBodyIndex :type Integer) (bFromSweep :type Boolean) (SweepResult :type "HitResult Structure (by ref)"))
  (bind _returnvalue (`GameplayStatics.GetPlayerCharacter` 0))
  (if (== OtherActor _returnvalue)
    (bind _asthird_person_character (cast `/Game/Blueprints/ThirdPersonBP/Blueprints/ThirdPersonCharacter` _returnvalue))
    (`/Game/Blueprints/ThirdPersonBP/Blueprints/ThirdPersonCharacter.Update Health` _asthird_person_character 100.0)))

(fn `UserConstructionScript`)