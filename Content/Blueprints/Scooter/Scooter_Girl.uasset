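; Scooter_Girl is a scooter quest NPC that shows dialogue when the third-person character enters its DialogueRadius.
; Entering creates a DialogueWidget and adds it to the viewport, while leaving removes it and sets GivenQuest.
; Tick separately refreshes the scooter quest text every frame on the Widget component's own dialogue widget, not the viewport instance.
; The Interact event is empty.
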(event `/Game/Blueprints/Interfaces/InteractInterface.Interact`
  (params (Interacter :type "Actor Object Reference")))

(event `self.DialogueRadius.OnComponentBeginOverlap`
  (params (OverlappedComponent :type "PrimitiveComponent Object Reference") (OtherActor :type "Actor Object Reference") (OtherComp :type "PrimitiveComponent Object Reference") (OtherBodyIndex :type Integer) (bFromSweep :type Boolean) (SweepResult :type "HitResult Structure (by ref)"))
  (`/Engine/EditorBlueprintResources/StandardMacros.IsValid` (`GameplayStatics.GetPlayerController` 0)
    (:`Is Valid`
      (cast `/Game/Blueprints/ThirdPersonBP/Blueprints/ThirdPersonCharacter` OtherActor)
      (`self.Show Dialogue`))))

(event `self.DialogueRadius.OnComponentEndOverlap`
  (params (OverlappedComponent :type "PrimitiveComponent Object Reference") (OtherActor :type "Actor Object Reference") (OtherComp :type "PrimitiveComponent Object Reference") (OtherBodyIndex :type Integer))
  (`/Engine/EditorBlueprintResources/StandardMacros.IsValid` (`GameplayStatics.GetPlayerController` 0)
    (:`Is Valid`
      (cast `/Game/Blueprints/ThirdPersonBP/Blueprints/ThirdPersonCharacter` OtherActor)
      (`self.Hide Dialogue`)
      (if (not (`self.bGivenQuest?`))
        (set `self.bGivenQuest?` true)))))

(event `self.ReceiveTick`
  (params (DeltaSeconds :type "Float (single-precision)"))
  (`self.Update Scooter Dialogue Text`))

(fn `Hide Dialogue`
  (`Widget.RemoveFromParent` (`self.DialogueWidget`)))

(fn `Show Dialogue`
  (`/Engine/EditorBlueprintResources/StandardMacros.IsValid` null
    (:`Is Valid`
      (bind _returnvalue (`|CreateWidget` "/Game/Blueprints/UI/UI_Dialog/DialogueWidget.DialogueWidget_C" null null))
      (bind _output_get (set `self.DialogueWidget` _returnvalue))
      (`UserWidget.AddToViewport` _returnvalue 0)
      (`UserWidget.AddToViewport` _output_get 0))))

(fn `Update Scooter Dialogue Text`
  (bind _asdialogue_widget (cast `/Game/Blueprints/UI/UI_Dialog/DialogueWidget` (`WidgetComponent.GetUserWidgetObject` (`self.Widget`))))
  (`/Game/Blueprints/UI/UI_Dialog/DialogueWidget.Update Scooter Quest Dialogue` _asdialogue_widget))

(fn `UserConstructionScript`)