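; Ice monster dummy Blueprint that shows a distance-scaled widget based on the player's key progress.
; A looping timer started on BeginPlay updates visibility from the player controller, showing the widget with the Flower key and hiding it once the Ice key is held.
; While visible, it measures distance to the player and enlarges the widget's draw size in steps as the player approaches, leaving it unchanged at closest range.
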(event `self.ReceiveBeginPlay`
  (`parent.ReceiveBeginPlay`)
  (bind _asnew_player_controller (cast `/Game/Blueprints/ThirdPersonBP/Blueprints/NewPlayerController` (`GameplayStatics.GetPlayerController` 0)))
  (set `self.As New Player Controller` _asnew_player_controller)
  (`KismetSystemLibrary.K2_SetTimerDelegate` (delegate `Widget_Range_Timer`) 0.2 true))

(event `Widget_Range_Timer`
  (`self.Widget_Visibility_Check`)
  (if (`SceneComponent.IsVisible` (`self.Widget`))
    (`self.Widget_Check_Range`)
    (`self.Widget_Scaling`)))

(event `Widget_Scaling`
  ;[1 1 1] Scaling
  (if (`SceneComponent.IsVisible` (`self.Widget`))
    (if (< (`self.RangeToPlayer`) 3000.0)
      (if (< (`self.RangeToPlayer`) 2000.0)
        (if (< (`self.RangeToPlayer`) 1000.0)
          (if (not (< (`self.RangeToPlayer`) 500.0))
            (`WidgetComponent.SetDrawSize` (`self.Widget`) (100.0 100.0)))
          (else
            (`WidgetComponent.SetDrawSize` (`self.Widget`) (90.0 90.0))))
        (else
          (`WidgetComponent.SetDrawSize` (`self.Widget`) (50.0 50.0))))
      (else
        (`WidgetComponent.SetDrawSize` (`self.Widget`) (30.0 30.0))))))

(event `Widget_Visibility_Check`
  (bind _as_new_player_controller (`self.As New Player Controller`))
  (bind _widget (`self.Widget`))
  (`|ExecutionSequence`
    (:`then_0`
      (if (`/Game/Blueprints/ThirdPersonBP/Blueprints/NewPlayerController.hasFlowerKey` _as_new_player_controller)
        (`SceneComponent.SetVisibility` _widget true false)))
    (:`then_1`
      (if (`/Game/Blueprints/ThirdPersonBP/Blueprints/NewPlayerController.hasIceKey` _as_new_player_controller)
        (`SceneComponent.SetVisibility` _widget false false)))))

(event `Widget_Check_Range`
  (set `self.RangeToPlayer` (`self.GetDistanceTo` (`GameplayStatics.GetPlayerCharacter` 0) self)))

(fn `UserConstructionScript`
  (`parent.UserConstructionScript`))