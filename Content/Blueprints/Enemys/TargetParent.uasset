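; TargetParent is the parent actor for clickable enemy targets, handling single-target selection and health.
; A left click stores it as the player controller's CurrentTarget, clears the previous target, shows a selection decal and refreshes the target frame UI.
; Damage updates current and normalized health, then either calls TargetDamaged or destroys the actor at zero.
; Destruction also destroys attached actors and, if selected, clears selection and notifies the controller.
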(event `ClearSelection`
  ;[1 1 1] ClearSelection
  (bind _asnew_player_controller (cast `/Game/Blueprints/ThirdPersonBP/Blueprints/NewPlayerController` (`GameplayStatics.GetPlayerController` 0)))
  (`/Game/Blueprints/ThirdPersonBP/Blueprints/NewPlayerController.ClearSelectedTarget` _asnew_player_controller)
  (`SceneComponent.SetVisibility` (`self.SelectionDecal`) false false)
  (set `self.IsSelected` false))

(event `ToggleSelection`
  (bind _selectiondecal (`self.SelectionDecal`))
  ;[1 1 1] Selection Toggle
  (if (`self.IsSelected`)
    (`SceneComponent.SetVisibility` _selectiondecal false false)
    (set `self.IsSelected` false)
    (else
      (`SceneComponent.SetVisibility` _selectiondecal true false)
      (set `self.IsSelected` true))))

(event `self.ReceiveActorOnClicked`
  (params (ButtonPressed :type "Key Structure"))
  ;[1 1 1] TargetOnClick
  (if (== ButtonPressed "LeftMouseButton")
    (`self.TargetTarget`)))

(event `TargetTarget`
  ;[1 1 1] TargetOnClick
  (if (not (`self.IsSelected`))
    (bind _asnew_player_controller (cast `/Game/Blueprints/ThirdPersonBP/Blueprints/NewPlayerController` (`GameplayStatics.GetPlayerController` 0)))
    (bind _currenttarget (`/Game/Blueprints/ThirdPersonBP/Blueprints/NewPlayerController.CurrentTarget` _asnew_player_controller)
      (:`then`
        (`self.ClearSelection` _currenttarget))
      (:`else`
        _))
    (set `/Game/Blueprints/ThirdPersonBP/Blueprints/NewPlayerController.CurrentTarget` self _asnew_player_controller)
    (`self.ToggleSelection`)
    ;[1 1 1] Update TargetFrame
    (bind _asthird_person_character (cast `/Game/Blueprints/ThirdPersonBP/Blueprints/ThirdPersonCharacter` (`GameplayStatics.GetPlayerCharacter` 0)))
    (`/Game/Blueprints/UI/UI_Target/Targetframe.UpdateTargetUI` (`/Game/Blueprints/UI/UI_Player/Player_UI.Targetframe` (`/Game/Blueprints/ThirdPersonBP/Blueprints/ThirdPersonCharacter.UI_Ref` _asthird_person_character)))))

(event `self.ReceiveDestroyed`
  ;[1 1 1] Clear Target On Destroy If Selected
  (for _array_element (`self.GetAttachedActors` true)
    (`self.K2_DestroyActor` _array_element))
  (if (`self.IsSelected`)
    (`self.ClearSelection`)
    (bind _asnew_player_controller (cast `/Game/Blueprints/ThirdPersonBP/Blueprints/NewPlayerController` (`GameplayStatics.GetPlayerController` 0)))
    (`/Game/Blueprints/ThirdPersonBP/Blueprints/NewPlayerController.CurrentTargetValid` _asnew_player_controller)))

(event `self.ReceiveBeginPlay`
  (set `self.TargetHealth_Current` (`self.TargetHealth_Max`)))

(event `self.ReceiveAnyDamage`
  (params (Damage :type "Float (single-precision)") (DamageType :type "DamageType Object Reference") (InstigatedBy :type "Controller Object Reference") (DamageCauser :type "Actor Object Reference"))
  (if (<= (`self.TargetHealth_Current`) 0.0)
    (`self.K2_DestroyActor`)
    (else
      (bind _output_get (set `self.TargetHealth_Current` (- (`self.TargetHealth_Current`) Damage)))
      (set `self.TargetHealth_Normalized` (`KismetMathLibrary.NormalizeToRange` _output_get 0.0 (`self.TargetHealth_Max`)))
      (if (<= (`self.TargetHealth_Current`) 0.0)
        (`self.K2_DestroyActor`)
        (else
          (`self.TargetDamaged`))))))

(fn `UserConstructionScript`)